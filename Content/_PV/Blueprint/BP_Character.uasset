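; BP_Character is a player character blueprint with mouse-cursor input and three abilities: sprint, guard and attack.
; On BeginPlay it shows the cursor, sets Game and UI input locked to the viewport, and grants the abilities through its AbilitySystemComp.
; MouseInGround line-traces the Visibility channel from the follow camera along the deprojected cursor direction and returns the hit under the mouse.
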(event `self.ReceiveBeginPlay`
  (bind _returnvalue (`GameplayStatics.GetPlayerController` 0))
  (bind _abilitysystemcomp (`self.AbilitySystemComp`))
  (set `PlayerController.bShowMouseCursor` true _returnvalue)
  (`WidgetBlueprintLibrary.SetInputMode_GameAndUIEx` _returnvalue null "LockAlways" false)
  (`PVAbilitySystemComp.AddAbility` _abilitysystemcomp null "/Game/_PV/Blueprint/Abilities/BP_Sprint.BP_Sprint_C")
  (`PVAbilitySystemComp.AddAbility` _abilitysystemcomp null "/Game/_PV/Blueprint/Abilities/BP_Guard.BP_Guard_C")
  (`PVAbilitySystemComp.AddAbility` _abilitysystemcomp null "/Game/_PV/Blueprint/Abilities/BP_Attack.BP_Attack_C"))

(fn `Mouse In Ground`
  (returns (OutHit :type "HitResult Structure"))
  (bind _returnvalue (`SceneComponent.K2_GetComponentLocation` (`self.FollowCamera`)))
  (bind _outhit (`KismetSystemLibrary.LineTraceSingle` _returnvalue (+ _returnvalue (* (`.WorldDirection` (`PlayerController.DeprojectMousePositionToWorld` (`GameplayStatics.GetPlayerController` 0))) 3500)) "TraceTypeQuery1"))
  (return _outhit))

(fn `UserConstructionScript`)